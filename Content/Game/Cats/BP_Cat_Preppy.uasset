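; Preppy cat variant, a child Blueprint that tags itself as "Preppy" and supplies that cat's matching rule and sprites.
; CheckMatch accepts another cat whose type is Polite, Jock or the same as its own.
; Sit, fail, success and cry overrides swap the Paper2D sprite, with sit and cry also calling the parent.
; Crying currently uses the same sprite whether sitting or standing.
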(event EventBeginPlay)

(event Collision|EventActorBeginOverlap
  (params (OtherActor :type Actor%20Object%20Reference)))

(event EventTick
  (params (DeltaSeconds :type Float%20%28single-precision%29)))

(fn ConstructionScript
  (Variables|Default|SetCatType (Utilities|String|MakeLiteralString "Preppy")))

(fn CheckMatch
  (params (OtherCat :type BP%20Cat%20Object%20Reference))
  (if (Utilities|Enum|Equal(Enum) (Variables|/Game/Game/Cats/BP_Cat.BP_Cat_C|GetCatType OtherCat) (Utilities|String|MakeLiteralString "Polite"))
    (return true)
    (elif (Utilities|Enum|Equal(Enum) (Variables|/Game/Game/Cats/BP_Cat.BP_Cat_C|GetCatType OtherCat) (Variables|Default|GetCatType))
      (return true)
      (else
        (return (Utilities|Enum|Equal(Enum) (Variables|/Game/Game/Cats/BP_Cat.BP_Cat_C|GetCatType OtherCat) (Utilities|String|MakeLiteralString "Jock")))))))

(fn SitDown
  (Rendering|Components|Sprite|SetSprite (Variables|Default|GetPaperSprite) "/Game/Assets/New_Cats/Preppy_Cat_Sit_Sprite.Preppy_Cat_Sit_Sprite")
  (|CallParentFunction))

(fn OnFail
  (Rendering|Components|Sprite|SetSprite (Variables|Default|GetPaperSprite) "/Game/Assets/Cats_Failed_Match/Preppy_Cat_Fail_Sprite.Preppy_Cat_Fail_Sprite"))

(fn OnSuccess
  (Rendering|Components|Sprite|SetSprite (Variables|Default|GetPaperSprite) "/Game/Assets/Cats_Successful_Match/Preppy_Cat_Success_Sprite.Preppy_Cat_Success_Sprite"))

(fn StartCrying
  (bind _papersprite (Variables|Default|GetPaperSprite))
  (if (Variables|Default|GetIsSitting)
    (Rendering|Components|Sprite|SetSprite _papersprite "/Game/Assets/Cats_Cry_Leaving/Preppy_Cat_Cry_1_Sprite.Preppy_Cat_Cry_1_Sprite") ; Should be sitting sprite
    (else
      (Rendering|Components|Sprite|SetSprite _papersprite "/Game/Assets/Cats_Cry_Leaving/Preppy_Cat_Cry_1_Sprite.Preppy_Cat_Cry_1_Sprite") ; Should be standing sprite
    ))
  (|CallParentFunction))