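; BP_Cat_Goth is the Goth cat variant, defining which cats it matches and which sprites it shows.
; The construction script sets its CatType, and CheckMatch accepts another cat that is Polite, Goth or Pastel.
; OnFail, OnSuccess and SitDown swap the Paper2D sprite, with SitDown also calling the parent implementation.
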(event EventBeginPlay)

(event Collision|EventActorBeginOverlap
  (params (OtherActor :type Actor%20Object%20Reference)))

(event EventTick
  (params (DeltaSeconds :type Float%20%28single-precision%29)))

(fn ConstructionScript
  (Variables|Default|SetCatType (Utilities|String|MakeLiteralString "Goth")))

(fn CheckMatch
  (params (OtherCat :type BP%20Cat%20Object%20Reference))
  (if (Utilities|Enum|Equal(Enum) (Variables|/Game/Game/Cats/BP_Cat.BP_Cat_C|GetCatType OtherCat) (Utilities|String|MakeLiteralString "Polite"))
    (return true)
    (elif (Utilities|Enum|Equal(Enum) (Variables|/Game/Game/Cats/BP_Cat.BP_Cat_C|GetCatType OtherCat) (Variables|Default|GetCatType))
      (return true)
      (else
        (return (Utilities|Enum|Equal(Enum) (Variables|/Game/Game/Cats/BP_Cat.BP_Cat_C|GetCatType OtherCat) (Utilities|String|MakeLiteralString "Pastel")))))))

(fn OnFail
  (Rendering|Components|Sprite|SetSprite (Variables|Default|GetPaperSprite) "/Game/Assets/Cats_Failed_Match/Goth_Cat_Fail_Sprite.Goth_Cat_Fail_Sprite"))

(fn OnSuccess
  (Rendering|Components|Sprite|SetSprite (Variables|Default|GetPaperSprite) "/Game/Assets/Cats_Successful_Match/Goth_Cat_Success_Sprite.Goth_Cat_Success_Sprite"))

(fn SitDown
  (Rendering|Components|Sprite|SetSprite (Variables|Default|GetPaperSprite) "/Game/Assets/New_Cats/Goth_Cat_Sit_Sprite.Goth_Cat_Sit_Sprite")
  (|CallParentFunction))