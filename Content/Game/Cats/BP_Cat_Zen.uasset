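; BP_Cat_Zen is the Zen cat, one cat type in what appears to be a matching game.
; Its construction script sets CatType to "Zen".
; CheckMatch accepts another cat whose type is either Polite or the same as its own.
; SitDown, OnFail and OnSuccess each swap the Paper2D sprite to the matching Zen pose; the event graph holds only disabled stubs.
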(event EventBeginPlay)

(event Collision|EventActorBeginOverlap
  (params (OtherActor :type Actor%20Object%20Reference)))

(event EventTick
  (params (DeltaSeconds :type Float%20%28single-precision%29)))

(fn ConstructionScript
  (Variables|Default|SetCatType (Utilities|String|MakeLiteralString "Zen")))

(fn CheckMatch
  (params (OtherCat :type BP%20Cat%20Object%20Reference))
  (if (Utilities|Enum|Equal(Enum) (Variables|/Game/Game/Cats/BP_Cat.BP_Cat_C|GetCatType OtherCat) (Utilities|String|MakeLiteralString "Polite"))
    (return true)
    (else
      (return (Utilities|Enum|Equal(Enum) (Variables|/Game/Game/Cats/BP_Cat.BP_Cat_C|GetCatType OtherCat) (Variables|Default|GetCatType))))))

(fn SitDown
  (Rendering|Components|Sprite|SetSprite (Variables|Default|GetPaperSprite) "/Game/Assets/New_Cats/Zen_Cat_Sit_Sprite.Zen_Cat_Sit_Sprite"))

(fn OnFail
  (Rendering|Components|Sprite|SetSprite (Variables|Default|GetPaperSprite) "/Game/Assets/Cats_Failed_Match/Zen_Cat_Fail_Sprite.Zen_Cat_Fail_Sprite"))

(fn OnSuccess
  (Rendering|Components|Sprite|SetSprite (Variables|Default|GetPaperSprite) "/Game/Assets/Cats_Successful_Match/Zen_Cat_Success_Sprite.Zen_Cat_Success_Sprite"))