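; BP_Cat_Snob is the Snob cat type, tagged by setting its CatType string in the construction script.
; CheckMatch accepts another cat whose type is Polite or the same as its own, comparing CatType strings.
; SitDown swaps the Paper2D sprite to a temporary sitting-cat sprite.
; The event graph holds only disabled default events, so it adds no runtime event logic.
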(event EventBeginPlay
  (|CallParentFunction) ; This node is disabled and will not be called.\nDrag off pins to build functionality.
)

(event Collision|EventActorBeginOverlap
  (params (OtherActor :type Actor%20Object%20Reference))
  (|CallParentFunction OtherActor) ; This node is disabled and will not be called.\nDrag off pins to build functionality.
)

(event EventTick
  (params (DeltaSeconds :type Float%20%28single-precision%29))
  (|CallParentFunction DeltaSeconds) ; This node is disabled and will not be called.\nDrag off pins to build functionality.
)

(fn ConstructionScript
  (Variables|Default|SetCatType (Utilities|String|MakeLiteralString "Snob")))

(fn CheckMatch
  (params (OtherCat :type BP%20Cat%20Object%20Reference))
  (if (Utilities|Enum|Equal(Enum) (Variables|/Game/Game/Cats/BP_Cat.BP_Cat_C|GetCatType OtherCat) (Utilities|String|MakeLiteralString "Polite"))
    (return true)
    (else
      (return (Utilities|Enum|Equal(Enum) (Variables|/Game/Game/Cats/BP_Cat.BP_Cat_C|GetCatType OtherCat) (Variables|Default|GetCatType))))))

(fn SitDown
  (Rendering|Components|Sprite|SetSprite (Variables|Default|GetPaperSprite) "/Game/Assets/Cats/Temporary_Sitting_Cat_Sprite.Temporary_Sitting_Cat_Sprite"))