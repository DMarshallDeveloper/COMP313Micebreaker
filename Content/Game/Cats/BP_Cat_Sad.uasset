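; BP_Cat_Sad is the Sad cat variant in a cat-matching game, tagging its CatType as "Sad" in the construction script.
; CheckMatch accepts another cat that is either Polite or the same type.
; SitDown, OnFail and OnSuccess swap the PaperSprite to sitting, red and green sprites, with the latter two using Polite cat art.
; Its event graph holds only disabled stub events.
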(event EventBeginPlay)

(event Collision|EventActorBeginOverlap
  (params (OtherActor :type Actor%20Object%20Reference)))

(event EventTick
  (params (DeltaSeconds :type Float%20%28single-precision%29)))

(fn ConstructionScript
  (Variables|Default|SetCatType (Utilities|String|MakeLiteralString "Sad")))

(fn CheckMatch
  (params (OtherCat :type BP%20Cat%20Object%20Reference))
  (if (Utilities|Enum|Equal(Enum) (Variables|/Game/Game/Cats/BP_Cat.BP_Cat_C|GetCatType OtherCat) (Utilities|String|MakeLiteralString "Polite"))
    (return true)
    (else
      (return (Utilities|Enum|Equal(Enum) (Variables|/Game/Game/Cats/BP_Cat.BP_Cat_C|GetCatType OtherCat) (Variables|Default|GetCatType))))))

(fn SitDown
  (Rendering|Components|Sprite|SetSprite (Variables|Default|GetPaperSprite) "/Game/Assets/Cats/Temporary_Sitting_Cat_Sprite.Temporary_Sitting_Cat_Sprite"))

(fn OnFail
  (Rendering|Components|Sprite|SetSprite (Variables|Default|GetPaperSprite) "/Game/Assets/Red_Green_Cats/Red_Polite_Cat_SIt_Sprite.Red_Polite_Cat_SIt_Sprite"))

(fn OnSuccess
  (Rendering|Components|Sprite|SetSprite (Variables|Default|GetPaperSprite) "/Game/Assets/Red_Green_Cats/Green_Polite_Cat_Sit_Sprite.Green_Polite_Cat_Sit_Sprite"))