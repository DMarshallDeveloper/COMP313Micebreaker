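; BP_Cat_Jock is the Jock cat variant, a child Blueprint that sets its CatType to "Jock" in the construction script.
; CheckMatch accepts another cat whose type is Polite, Preppy or the same as its own.
; State functions swap the Paper2D sprite for selection, match results, sitting and crying, with separate sitting and standing cry sprites.
; SitDown also calls its parent, while StartCrying does so only when the cat is sitting.
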(event EventBeginPlay
  (|CallParentFunction) ; This node is disabled and will not be called.\nDrag off pins to build functionality.
)

(event Collision|EventActorBeginOverlap
  (params (OtherActor :type Actor%20Object%20Reference))
  (|CallParentFunction OtherActor) ; This node is disabled and will not be called.\nDrag off pins to build functionality.
)

(event EventTick
  (params (DeltaSeconds :type Float%20%28single-precision%29))
  (|CallParentFunction DeltaSeconds) ; This node is disabled and will not be called.\nDrag off pins to build functionality.
)

(fn ConstructionScript
  (Variables|Default|SetCatType (Utilities|String|MakeLiteralString "Jock")))

(fn CheckMatch
  (params (OtherCat :type BP%20Cat%20Object%20Reference))
  (if (Utilities|Enum|Equal(Enum) (Variables|/Game/Game/Cats/BP_Cat.BP_Cat_C|GetCatType OtherCat) (Utilities|String|MakeLiteralString "Polite"))
    (return true)
    (elif (Utilities|Enum|Equal(Enum) (Variables|/Game/Game/Cats/BP_Cat.BP_Cat_C|GetCatType OtherCat) (Variables|Default|GetCatType))
      (return true)
      (else
        (return (Utilities|Enum|Equal(Enum) (Variables|/Game/Game/Cats/BP_Cat.BP_Cat_C|GetCatType OtherCat) (Utilities|String|MakeLiteralString "Preppy")))))))

(fn SitDown
  (Rendering|Components|Sprite|SetSprite (Variables|Default|GetPaperSprite) "/Game/Assets/New_Cats/Jock_Cat_Sit_Sprite.Jock_Cat_Sit_Sprite")
  (|CallParentFunction))

(fn MatchFail
  (Rendering|Components|Sprite|SetSprite (Variables|Default|GetPaperSprite) "/Game/Assets/Cats_Failed_Match/Jock_Cat_Fail_Sprite.Jock_Cat_Fail_Sprite"))

(fn MatchSuccess
  (Rendering|Components|Sprite|SetSprite (Variables|Default|GetPaperSprite) "/Game/Assets/Cats_Successful_Match/Jock_Cat_Success_Sprite.Jock_Cat_Success_Sprite"))

(fn CatDeselected
  (Rendering|Components|Sprite|SetSprite (Variables|Default|GetPaperSprite) "/Game/Assets/New_Cats/Jock_Cat_1_Sprite.Jock_Cat_1_Sprite"))

(fn CatSelected
  (Rendering|Components|Sprite|SetSprite (Variables|Default|GetPaperSprite) "/Game/Assets/Cats_Highlighted/Jock_Cat_Highlighted_Sprite.Jock_Cat_Highlighted_Sprite"))

(fn StartCrying
  (bind _papersprite (Variables|Default|GetPaperSprite))
  (if (Variables|Default|GetIsSitting)
    (Rendering|Components|Sprite|SetSprite _papersprite "/Game/Assets/Cats_Cry_Leaving/Cats_Cry_Sit/Jock_Cat_Cry_Sit_1_Sprite.Jock_Cat_Cry_Sit_1_Sprite") ; Should be sitting sprite
    (|CallParentFunction)
    (else
      (Rendering|Components|Sprite|SetSprite _papersprite "/Game/Assets/Cats_Cry_Leaving/Jock_Cat_Cry_1_Sprite.Jock_Cat_Cry_1_Sprite") ; Should be standing sprite
    )))