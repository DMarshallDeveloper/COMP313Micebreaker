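; BP_Cat is a clickable cat actor that passes itself to MainGameInstance's ClickSelect when clicked.
; It takes its starting patience from the game instance's Level1Patience and counts it down every Tick, showing a "Leaving in" seconds label while above one second.
; The one-second label and the destroy call are unwired, so nothing happens at zero, and CheckMatch is a stub that always returns false.
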(event EventTick
  (params (DeltaSeconds :type Float%20%28single-precision%29))
  (bind _output_get (Variables|Default|SetCurrentPatience (- (Variables|Default|GetCurrentPatience) DeltaSeconds)))
  (if (not (<= _output_get 0.0))
    (if (> (Class|KismetMathLibrary|Round64 (Variables|Default|GetCurrentPatience)) 1)
      (Rendering|Components|TextRender|SetText (Variables|Default|GetPatience) (Utilities|Text|ToText(String) (Utilities|String|Append "Leaving in:  " (Utilities|String|ToString(Text) (Utilities|Text|ToText(String) (Class|KismetMathLibrary|Round64 (Variables|Default|GetCurrentPatience)))) " Seconds")))
      (elif (== (Class|KismetMathLibrary|Round64 (Variables|Default|GetCurrentPatience)) 1)
        _))))

(event MouseInput|EventActorOnClicked
  (params (ButtonPressed :type Key%20Structure :default "None"))
  (bind _asmain_game_instance (Utilities|Casting|CastToMainGameInstance (Game|GetGameInstance)))
  (Default|ClickSelect _asmain_game_instance self))

(event EventBeginPlay
  (bind _asmain_game_instance (Utilities|Casting|CastToMainGameInstance (Game|GetGameInstance)))
  (Variables|Default|SetCurrentPatience (Variables|/Game/Game/MainGameInstance.MainGameInstance_C|GetLevel1Patience _asmain_game_instance)))

(fn ConstructionScript)

(fn CheckMatch
  (params (OtherCat :type BP%20Cat%20Object%20Reference))
  (return false))