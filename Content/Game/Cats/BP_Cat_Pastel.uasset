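; BP_Cat_Pastel is the Pastel cat variant, a child Blueprint that supplies this type's sprites and matching rules.
; The construction script sets CatType to Pastel, and CheckMatch accepts Polite, Goth or same-type cats.
; Overridden state functions swap the Paper2D sprite for selection, match results, sitting and crying.
; SitDown also calls the parent, while StartCrying does so only when the cat is sitting.
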(event EventBeginPlay)

(event Collision|EventActorBeginOverlap
  (params (OtherActor :type Actor%20Object%20Reference)))

(event EventTick
  (params (DeltaSeconds :type Float%20%28single-precision%29)))

(fn ConstructionScript
  (Variables|Default|SetCatType (Utilities|String|MakeLiteralString "Pastel")))

(fn CheckMatch
  (params (OtherCat :type BP%20Cat%20Object%20Reference))
  (if (Utilities|Enum|Equal(Enum) (Variables|/Game/Game/Cats/BP_Cat.BP_Cat_C|GetCatType OtherCat) (Utilities|String|MakeLiteralString "Polite"))
    (return true)
    (elif (Utilities|Enum|Equal(Enum) (Variables|/Game/Game/Cats/BP_Cat.BP_Cat_C|GetCatType OtherCat) (Variables|Default|GetCatType))
      (return true)
      (else
        (return (Utilities|Enum|Equal(Enum) (Variables|/Game/Game/Cats/BP_Cat.BP_Cat_C|GetCatType OtherCat) (Utilities|String|MakeLiteralString "Goth")))))))

(fn SitDown
  (Rendering|Components|Sprite|SetSprite (Variables|Default|GetPaperSprite) "/Game/Assets/New_Cats/Pastel_Cat_Sit_Sprite.Pastel_Cat_Sit_Sprite")
  (|CallParentFunction))

(fn MatchSuccess
  (Rendering|Components|Sprite|SetSprite (Variables|Default|GetPaperSprite) "/Game/Assets/Cats_Successful_Match/Pastel_Cat_Success_Sprite.Pastel_Cat_Success_Sprite"))

(fn MatchFail
  (Rendering|Components|Sprite|SetSprite (Variables|Default|GetPaperSprite) "/Game/Assets/Cats_Failed_Match/Pastel_Cat_Fail_Sprite.Pastel_Cat_Fail_Sprite"))

(fn CatDeselected
  (Rendering|Components|Sprite|SetSprite (Variables|Default|GetPaperSprite) "/Game/Assets/New_Cats/Pastel_Cat_1_Sprite.Pastel_Cat_1_Sprite"))

(fn CatSelected
  (Rendering|Components|Sprite|SetSprite (Variables|Default|GetPaperSprite) "/Game/Assets/Cats_Highlighted/Pastel_Cat_Highlighted_Sprite.Pastel_Cat_Highlighted_Sprite"))

(fn StartCrying
  (bind _papersprite (Variables|Default|GetPaperSprite))
  (if (Variables|Default|GetIsSitting)
    (Rendering|Components|Sprite|SetSprite _papersprite "/Game/Assets/Cats_Cry_Leaving/Cats_Cry_Sit/Pastel_Cat_Cry_Sit_1_Sprite.Pastel_Cat_Cry_Sit_1_Sprite") ; Should be sitting sprite
    (|CallParentFunction)
    (else
      (Rendering|Components|Sprite|SetSprite _papersprite "/Game/Assets/Cats_Cry_Leaving/Pastel_Cat_Cry_1_Sprite.Pastel_Cat_Cry_1_Sprite") ; Should be standing sprite
    )))