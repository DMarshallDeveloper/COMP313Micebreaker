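; Cat Blueprint for the Slob personality type, defining which other cats count as a match for it.
; The construction script sets CatType to "Slob".
; CheckMatch compares the other cat's CatType string and returns true for Polite, the same type, or Hipster, and false otherwise.
; The event graph holds only disabled placeholder events.
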(event EventBeginPlay)

(event Collision|EventActorBeginOverlap
  (params (OtherActor :type Actor%20Object%20Reference)))

(event EventTick
  (params (DeltaSeconds :type Float%20%28single-precision%29)))

(fn ConstructionScript
  (Variables|Default|SetCatType (Utilities|String|MakeLiteralString "Slob")))

(fn CheckMatch
  (params (OtherCat :type BP%20Cat%20Object%20Reference))
  (if (Utilities|Enum|Equal(Enum) (Variables|/Game/Game/Cats/BP_Cat.BP_Cat_C|GetCatType OtherCat) (Utilities|String|MakeLiteralString "Polite"))
    (return true)
    (elif (Utilities|Enum|Equal(Enum) (Variables|/Game/Game/Cats/BP_Cat.BP_Cat_C|GetCatType OtherCat) (Variables|Default|GetCatType))
      (return true)
      (else
        (return (Utilities|Enum|Equal(Enum) (Variables|/Game/Game/Cats/BP_Cat.BP_Cat_C|GetCatType OtherCat) (Utilities|String|MakeLiteralString "Hipster")))))))