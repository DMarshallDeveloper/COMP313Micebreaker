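; Shop item manager that creates and tracks the purchasable decor items: tables, windows, seats, doors, walls, floors and plants.
; On Initialize it constructs animated, window or still item objects from data arrays, passing each the GameInstance.
; Items are stored per group in AllItems for lookup through GetItems.
; Default-owned items fill ActiveItems, one per group with later ones replacing earlier, and are activated once creation finishes.
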(fn Initialize
  (params (Game%20Instance :type Main%20Game%20Instance%20Object%20Reference))
  ;[1 1 1] Creates all of the items from item data
  (Variables|Default|SetGame%20Instance Game%20Instance)
  (Utilities|FlowControl|Sequence
    (:then_0
      (CallFunction|CreateAnimatedItems (Variables|ItemData|GetTables) "NewEnumerator0"))
    (:then_1
      (CallFunction|CreateWindowItems (Variables|ItemData|GetWindows)))
    (:then_2
      (CallFunction|CreateStillItems (Variables|ItemData|GetSeats) "NewEnumerator2")
      (CallFunction|CreateStillItems (Variables|ItemData|GetDoors) "NewEnumerator3")
      (CallFunction|CreateStillItems (Variables|ItemData|GetWalls) "NewEnumerator5")
      (CallFunction|CreateStillItems (Variables|ItemData|GetFloors) "NewEnumerator6")
      (CallFunction|CreateStillItems (Variables|ItemData|GetPlants) "NewEnumerator4"))
    (:then_3
      ;[1 1 1] Activate all items in use
      (bind _values (Utilities|Map|Values (Variables|Default|GetActive%20Items)))
      (for _array_element _values
        (Default|Activate _array_element)
        (Development|PrintString 0 (Utilities|GetDisplayName _array_element) false true "(R=0.000000,G=0.660000,B=1.000000,A=1.000000)" 1.0)))))

(fn AddItem
  (params (Group :type ItemGroup%20Enum :default "NewEnumerator0") (Item :type BP%20Item%20Object%20Reference))
  ;[1 1 1] Adds a BP_Item to the collection of all items
  (LocalVariables|SetItem%20Group Group)
  (bind _output_get (LocalVariables|SetTempArray (Utilities|Struct|BreakItems (.Value (Utilities|Map|Find (Variables|Default|GetAll%20Items) Group)))))
  (Utilities|Array|Add _output_get Item)
  (Utilities|Map|Add (Variables|Default|GetAll%20Items) (LocalVariables|GetItem%20Group) (Utilities|Struct|MakeItems (LocalVariables|GetTempArray))))

(fn CreateWindowItems
  (params (Window%20Items :type Array%20of%20Item%20Window%20Data%20Structures))
  ;[1 1 1] Constructs BP_Item_Window/s from window item data
  (for _array_element Window%20Items
    (bind _returnvalue (Game|ConstructObjectfromClass "/Game/Game/Shop/BP_Item_Window.BP_Item_Window_C" self (.LeftSprite (Utilities|Struct|BreakItemWindowData _array_element)) (.RightSprite (Utilities|Struct|BreakItemWindowData _array_element)) (.Price (Utilities|Struct|BreakItemWindowData _array_element)) (.Default (Utilities|Struct|BreakItemWindowData _array_element)) (.ShopIcon (Utilities|Struct|BreakItemWindowData _array_element)) (Variables|Default|GetGame%20Instance)))
    (CallFunction|AddItem "NewEnumerator1" _returnvalue)
    ;;[1 1 1] Set as active currently active item
    (if (Variables|/Game/Game/Shop/BP_Item.BP_Item_C|GetIs%20Owned _returnvalue)
      (Utilities|Map|Add (Variables|Default|GetActive%20Items) "NewEnumerator1" _returnvalue))))

(fn CreateStillItems
  (params (Items :type Array%20of%20Item%20Still%20Data%20Structures) (Group :type ItemGroup%20Enum :default "NewEnumerator0"))
  ;[1 1 1] Contructs a BP_Item that is not animated, from item data
  (LocalVariables|SetItemGroup Group)
  (for _array_element Items
    (bind _returnvalue (Game|ConstructObjectfromClass "/Game/Game/Shop/BP_Item_Still.BP_Item_Still_C" self (.Type (Utilities|Struct|BreakItemStillData _array_element)) (.Sprite (Utilities|Struct|BreakItemStillData _array_element)) (.Price (Utilities|Struct|BreakItemStillData _array_element)) (.Default (Utilities|Struct|BreakItemStillData _array_element)) (.ShopIcon (Utilities|Struct|BreakItemStillData _array_element)) (Variables|Default|GetGame%20Instance)))
    (CallFunction|AddItem (LocalVariables|GetItemGroup) _returnvalue)
    ;;[1 1 1] Set as active currently active item
    (if (Variables|/Game/Game/Shop/BP_Item.BP_Item_C|GetIs%20Owned _returnvalue)
      (Utilities|Map|Add (Variables|Default|GetActive%20Items) (LocalVariables|GetItemGroup) _returnvalue))))

(fn CreateAnimatedItems
  (params (Items :type Array%20of%20Item%20Animated%20Data%20Structures) (Group :type ItemGroup%20Enum :default "NewEnumerator0"))
  ;[1 1 1] Constructs BP_Item/s that are animated, from item data
  (LocalVariables|SetItem%20Group Group)
  (for _array_element Items
    (bind _returnvalue (Game|ConstructObjectfromClass "/Game/Game/Shop/BP_Item_Animated.BP_Item_Animated_C" self (.Flipbook (Utilities|Struct|BreakItemAnimatedData _array_element)) (.Type (Utilities|Struct|BreakItemAnimatedData _array_element)) (.Price (Utilities|Struct|BreakItemAnimatedData _array_element)) (.Default (Utilities|Struct|BreakItemAnimatedData _array_element)) (.ShopIcon (Utilities|Struct|BreakItemAnimatedData _array_element)) (Variables|Default|GetGame%20Instance)))
    (CallFunction|AddItem (LocalVariables|GetItem%20Group) _returnvalue)
    ;;[1 1 1] Set as active currently active item
    (if (Variables|/Game/Game/Shop/BP_Item.BP_Item_C|GetIs%20Owned _returnvalue)
      (Utilities|Map|Add (Variables|Default|GetActive%20Items) (LocalVariables|GetItem%20Group) _returnvalue))))

(fn GetItems
  (params (Item%20Group :type ItemGroup%20Enum :default "NewEnumerator0"))
  (bind _all_items (Variables|Default|GetAll%20Items))
  (bind (_value _returnvalue) (Utilities|Map|Find _all_items Item%20Group))
  ;[1 1 1] Gets all the items belonging to an item group
  (if _returnvalue
    (return (Utilities|Struct|BreakItems _value))))