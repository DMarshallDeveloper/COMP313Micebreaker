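; BP_Customizations stores the current 2D appearance for each customizable component type, as either a still sprite or an animated flipbook.
; It keeps two maps keyed by type, StillAppearances and AnimatedAppearances, with a getter and setter for each.
; Getters return null for missing types, and setters only overwrite existing keys, so each map's predefined keys decide which types belong to it.
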(fn GetAppearanceStill
  (params (Type :type ComponentType%20Enum :default "NewEnumerator1"))
  (bind _stillappearances (Variables|Default|GetStillAppearances))
  (bind (_value _returnvalue) (Utilities|Map|Find _stillappearances Type))
  ;[1 1 1] Gets the current appearance (Sprite) of a given component type. Returns null if not found
  (if _returnvalue
    (return _value)
    (else
      (return 0))))

(fn GetAppearanceAnimated
  (params (Component%20Type :type ComponentType%20Enum :default "NewEnumerator4"))
  (bind _animatedappearances (Variables|Default|GetAnimatedAppearances))
  (bind (_value _returnvalue) (Utilities|Map|Find _animatedappearances Component%20Type))
  ;[1 1 1] Gets the current appearance (FlipBook) of a given component type. Returns null if not found
  (if _returnvalue
    (return _value)
    (else
      (return 0))))

(fn SetAppearanceStill
  (params (Type :type ComponentType%20Enum :default "NewEnumerator1") (Sprite :type Paper%20Sprite%20Object%20Reference))
  ;[1 1 1] Sets a value (a flipbook) in StillAppearances, given a key
  (if (.ReturnValue (Utilities|Map|Find (Variables|Default|GetStillAppearances) Type))
    (Utilities|Map|Add (Variables|Default|GetStillAppearances) Type Sprite)))

(fn SetAppearanceAnimated
  (params (Type :type ComponentType%20Enum :default "NewEnumerator1") (Flipbook :type Paper%20Flipbook%20Object%20Reference))
  ;[1 1 1] Sets a value (a flipbook) in AnimatedAppearances, given a key
  (if (.ReturnValue (Utilities|Map|Find (Variables|Default|GetAnimatedAppearances) Type))
    (Utilities|Map|Add (Variables|Default|GetAnimatedAppearances) Type Flipbook)))