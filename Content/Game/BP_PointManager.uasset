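; Point manager that tracks points collected in a level and converts them into stars and coins.
; CalculateScore rates CurrentPoints against per-level thresholds for zero to three stars, then looks up that rating's coin value.
; It awards only the amount above what that level has already paid, so replays earn coins just for improvement.
; The award updates the level's CoinsEarned entry and BankBalance, and is returned with the star count.
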(fn CalculateScore
  (params (Level%20Number :type Integer))
  ;[1 1 1] Calculates the number of stars and coins earned based on the number of points collected in a level
  (bind _num_stars (CallFunction|CalculateStars Level%20Number))
  (bind _coins (CallFunction|CalculateCoins Level%20Number _num_stars))
  (CallFunction|UpdateCoinsEarned Level%20Number _coins)
  ;;[1 1 1] Add coins earned to bank
  (Variables|Default|SetBank%20Balance (+ (Variables|Default|GetBank%20Balance) _coins))
  (return _num_stars _coins))

(fn CalculateStars
  (params (Level%20Number :type Integer))
  (bind _thresholds (Variables|Default|GetThresholds))
  (bind _output (Utilities|Array|Get(acopy) _thresholds Level%20Number))
  (bind (_1star _2stars _3stars) (Utilities|Struct|BreakPointThreshold _output))
  ;[1 1 1] Calculates how many stars have been earnt based based on the level completed, and number of points earned
  (if (>= (Variables|Default|GetCurrent%20Points) _3stars)
    (return 3)
    (elif (>= (Variables|Default|GetCurrent%20Points) _2stars)
      (return 2)
      (elif (>= (Variables|Default|GetCurrent%20Points) _1star)
        (return 1)
        (else
          (return 0) ; failed
        )))))

(fn CalculateCoins
  (params (Level :type Integer) (Stars :type Integer))
  (bind _output_get (LocalVariables|SetDifference (- (.Value (Utilities|Map|Find (Variables|Default|GetStar%20Value) Stars)) (.Value (Utilities|Map|Find (Variables|Default|GetCoins%20Earned) Level)))))
  (if (<= _output_get 0)
    (return 0)
    (else
      (return (LocalVariables|GetDifference)))))

(fn UpdateCoinsEarned
  (params (Level%20Number :type Integer) (Coins%20Earned :type Integer))
  ;[1 1 1] Increments the total number of coins earned for a given level, by a given amount
  (Utilities|Map|Add (Variables|Default|GetCoins%20Earned) Level%20Number (+ (.Value (Utilities|Map|Find (Variables|Default|GetCoins%20Earned) Level%20Number)) Coins%20Earned)))

(fn AddPoints
  (params (Points :type Integer))
  (Variables|Default|SetCurrent%20Points (+ (Variables|Default|GetCurrent%20Points) Points)))