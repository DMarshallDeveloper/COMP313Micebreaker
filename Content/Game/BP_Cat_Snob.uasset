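; BP_Cat_Snob is the Snob variant of a cat actor, defining which other cats it matches with.
; The construction script runs the parent's, then sets CatType to "Snob".
; CheckMatch always rejects "Polite" cats and otherwise returns true only when the other cat's CatType equals its own.
; The event graph holds only disabled placeholder events.
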(event EventBeginPlay
  (|CallParentFunction) ; This node is disabled and will not be called.\nDrag off pins to build functionality.
)

(event Collision|EventActorBeginOverlap
  (params (OtherActor :type Actor%20Object%20Reference))
  (|CallParentFunction OtherActor) ; This node is disabled and will not be called.\nDrag off pins to build functionality.
)

(event EventTick
  (params (DeltaSeconds :type Float%20%28single-precision%29))
  (|CallParentFunction DeltaSeconds) ; This node is disabled and will not be called.\nDrag off pins to build functionality.
)

(fn ConstructionScript
  (|CallParentFunction)
  (Variables|Default|SetCatType (Utilities|String|MakeLiteralString "Snob")))

(fn CheckMatch
  (params (OtherCat :type BP%20Cat%20Object%20Reference))
  (if (Utilities|Enum|Equal(Enum) (Variables|/Game/Game/BP_Cat.BP_Cat_C|GetCatType OtherCat) (Utilities|String|MakeLiteralString "Polite"))
    (return false)
    (else
      (return (Utilities|Enum|Equal(Enum) (Variables|/Game/Game/BP_Cat.BP_Cat_C|GetCatType OtherCat) (Variables|Default|GetCatType))))))