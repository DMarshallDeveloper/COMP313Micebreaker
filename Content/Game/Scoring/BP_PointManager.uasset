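; Point manager that tracks level points, completed levels and the player's coin balance.
; CalculateScore turns current points into zero to three stars using per-level thresholds, then converts stars into coins added to the bank.
; A per-level map of coins already earned limits each payout to the improvement over previous attempts, so replays cannot farm coins.
; AddPoints accepts only positive values and triggers a pop-out on the level HUD.
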(fn CalculateScore
  (params (Level%20Number :type Integer))
  ;[1 1 1] Calculates the number of stars and coins earned based on the number of points collected in a level
  (bind _num_stars (CallFunction|CalculateStars Level%20Number))
  (bind _coins (CallFunction|CalculateCoins Level%20Number _num_stars))
  (CallFunction|UpdateCoinsEarned Level%20Number _coins)
  ;;[1 1 1] Add coins earned to bank
  (Variables|Default|SetBankBalance (+ (Variables|Default|GetBankBalance) _coins))
  (return _num_stars _coins (Variables|Default|GetCurrentPoints)))

(fn CalculateStars
  (params (Level%20Number :type Integer))
  (bind _thresholds (Variables|Default|GetThresholds))
  (bind _output (Utilities|Array|Get(acopy) _thresholds Level%20Number))
  (bind (_1star _2stars _3stars) (Utilities|Struct|BreakPointThreshold _output))
  ;[1 1 1] Calculates how many stars have been earnt based based on the level completed, and number of points earned
  (if (>= (Variables|Default|GetCurrentPoints) _3stars)
    (return 3)
    (elif (>= (Variables|Default|GetCurrentPoints) _2stars)
      (return 2)
      (elif (>= (Variables|Default|GetCurrentPoints) _1star)
        (return 1)
        (else
          (return 0) ; failed
        )))))

(fn CalculateCoins
  (params (Level :type Integer) (Stars :type Integer))
  (bind _output_get (LocalVariables|SetDifference (- (.Value (Utilities|Map|Find (Variables|Default|GetStarValue) Stars)) (.Value (Utilities|Map|Find (Variables|Default|GetCoinsEarned) Level)))))
  (if (<= _output_get 0)
    (return 0)
    (else
      (return (LocalVariables|GetDifference)))))

(fn UpdateCoinsEarned
  (params (Level%20Number :type Integer) (Earned :type Integer))
  ;[1 1 1] Increments the total number of coins earned for a given level, by a given amount
  (Utilities|Map|Add (Variables|Default|GetCoinsEarned) Level%20Number (+ (.Value (Utilities|Map|Find (Variables|Default|GetCoinsEarned) Level%20Number)) Earned)))

(fn AddPoints
  (params (Points :type Integer))
  (if (> Points 0)
    (Variables|Default|SetCurrentPoints (+ (Variables|Default|GetCurrentPoints) Points))
    (Default|PopOut (Variables|/Game/Game/MainGameInstance.MainGameInstance_C|GetLevelHUD (Variables|Default|GetGameInstance)))))

(fn SetLevelComplete
  (params (Level :type Integer))
  (Utilities|Map|Add (Variables|Default|GetCompletedLevels) Level true)
  (Development|PrintString 0 (Utilities|String|ToString(Integer) Level)))

(fn IsLevelCompleted
  (params (Level :type Integer))
  (return (.Value (Utilities|Map|Find (Variables|Default|GetCompletedLevels) Level))))