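; BP_RestaurantComponent is a restaurant piece whose 2D look follows the globally active item for its Type.
; On BeginPlay, SetAppearance asks the ItemManager in MainGameInstance for that active item.
; The IsAnimated flag selects whether the item is cast to BP_Item_Animated to set the FlipBook, or to BP_Item_Still to set the Sprite.
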(event EventBeginPlay
  (CallFunction|SetAppearance))

(event Collision|EventActorBeginOverlap
  (params (OtherActor :type Actor%20Object%20Reference)))

(event EventTick
  (params (DeltaSeconds :type Float%20%28single-precision%29)))

(fn ConstructionScript)

(fn SetAppearance
  ;[1 1 1] Applies global appearance to this restaurant component
  (bind _asmain_game_instance (Utilities|Casting|CastToMainGameInstance (Game|GetGameInstance)))
  (bind _newparam (Default|GetActiveItem (Variables|/Game/Game/MainGameInstance.MainGameInstance_C|GetItemManager _asmain_game_instance) (Variables|Type|GetType)))
  (if (Variables|Type|GetIsAnimated)
    (bind _asbp_item_animated (Utilities|Casting|CastToBP_Item_Animated _newparam))
    (Sprite|SetFlipbook (Variables|Default|GetFlipBook) (Variables|/Game/Game/Shop/BP_Item_Animated.BP_Item_Animated_C|GetFlipBook _asbp_item_animated))
    (else
      (bind _asbp_item_still (Utilities|Casting|CastToBP_Item_Still _newparam))
      (Rendering|Components|Sprite|SetSprite (Variables|Default|GetSprite) (Variables|/Game/Game/Shop/BP_Item_Still.BP_Item_Still_C|GetSprite _asbp_item_still)))))