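; BP_QueueManager runs the restaurant's queue of cats and registers itself with MainGameInstance on BeginPlay.
; Tick drives a timer that spawns the next cat from a temporary fixed sequence while the queue has room.
; A map stores each cat's slot, resolved to world space through hidden mesh components tagged by slot number.
; RemoveCat shifts the cats behind the gap forward and snaps them to their new spots.
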(event EventBeginPlay
  (Rendering|SetVisibility (Variables|Default|GetDefaultSceneRoot) false true)
  (bind _asmain_game_instance (Utilities|Casting|CastToMainGameInstance (Game|GetGameInstance)))
  (Variables|/Game/Game/MainGameInstance.MainGameInstance_C|SetQueueManager _asmain_game_instance self))

(event Collision|EventActorBeginOverlap
  (params (OtherActor :type Actor%20Object%20Reference)))

(event EventTick
  (params (DeltaSeconds :type Float%20%28single-precision%29))
  (CallFunction|UpdateTimer DeltaSeconds))

(fn ConstructionScript)

(fn RemoveCat
  (params (cat :type BP%20Cat%20Object%20Reference))
  ;[1 1 1] decremement length of queue
  (bind _result (Math|Integer|DecrementInt (Variables|Default|GetQueue%20Size))
    (:%20%20
      (Variables|Default|SetQueue%20Size _result)
      (LocalVariables|SetGapPosition (.Value (Utilities|Map|Find (Variables|Default|GetQueue) cat)))
      ;[1 1 1] Remove from queue map
      (Utilities|Map|Remove (Variables|Default|GetQueue) cat)
      (bind _keys (Utilities|Map|Keys (Variables|Default|GetQueue)))
      (for _array_element _keys ; Move all cats behind the \nqueue gap up a position
        ;[1 1 1] Move all cats that were behind the removed cat up a queue position (temp? add animation later)
        (if (> (.Value (Utilities|Map|Find (Variables|Default|GetQueue) _array_element)) (LocalVariables|GetGapPosition))
          (bind _result_2 (Math|Integer|DecrementInt (.Value (Utilities|Map|Find (Variables|Default|GetQueue) _array_element)))
            (:%20%20
              (Utilities|Map|Add (Variables|Default|GetQueue) _array_element _result_2)))))
      (CallFunction|UpdateWorldPositions))))

(fn UpdateTimer
  (params (Delta%20Time :type Float%20%28single-precision%29))
  ;[1 1 1] increment time
  (bind _output_get (Variables|Default|SetTime%20Elapsed (+ Delta%20Time (Variables|Default|GetTime%20Elapsed))))
  (if (> _output_get (Variables|Default|GetSpawn%20Time))
    (CallFunction|SpawnCat)))

(fn SpawnCat
  ;[1 1 1] Check that the queue isn't full
  (if (< (Variables|Default|GetQueue%20Size) (Variables|Default|GetQueue%20Limit))
    (if (not (== (Variables|Default|GetSequence%20Index) 11)) ; TEMPORARY
      (Variables|Default|SetTime%20Elapsed 0.0) ; reset time elapsed
      (bind _result (Math|Integer|IncrementInt (Variables|Default|GetQueue%20Size))
        (:%20%20
          (bind _output_get (LocalVariables|SetQueue%20Position _result))
          ;[1 1 1] Spawn and place cat in world
          (bind _position (CallFunction|GetWorldPosition _output_get))
          (bind _type (CallFunction|GetCatType))
          (bind _returnvalue (Game|SpawnActorfromClass _type (Math|Conversions|ToTransform(Vector) _position) "Undefined" 0 0))
          ;[1 1 1] Add the cat and its queue position to the queue map
          (Utilities|Map|Add (Variables|Default|GetQueue) _returnvalue (LocalVariables|GetQueue%20Position)))))))

(fn UpdateWorldPositions
  ;[1 1 1] Sets the world position of the cats in the queue, based on their position in the queue
  (bind _keys (Utilities|Map|Keys (Variables|Default|GetQueue)))
  (for _array_element _keys
    (bind _position (CallFunction|GetWorldPosition (.Value (Utilities|Map|Find (Variables|Default|GetQueue) _array_element))))
    (Transformation|SetActorLocation _array_element _position false false)))

(fn GetWorldPosition
  (params (Queue%20Position :type Integer))
  ;[1 1 1] Gets the world position, given a position in the queue
  (return (Transformation|GetWorldLocation (Utilities|Array|Get(acopy) (Actor|GetComponentsbyTag "/Script/Engine.MeshComponent" (Utilities|String|StringToName (Utilities|String|ToString(Integer) Queue%20Position)))))))

(fn GetCatType
  ;[1 1 1] Gets a type of cat from a determined sequence (Temporary)
  (bind _result (Math|Integer|IncrementInt (Variables|Default|GetSequence%20Index))
    (:%20%20
      (bind _output_get (Variables|Default|SetSequence%20Index _result))
      (return (Utilities|Array|Get(acopy) (Variables|Default|GetTemporary%20Sequence) (- _output_get 1))))))