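; Restaurant queue manager that spawns cats at the door and lines them up, registering itself with MainGameInstance.
; While unpaused, a Tick timer spawns cats up to the queue limit, picking types from cumulative probability intervals built by SetProbabilities.
; A map tracks each cat's position, resolved to world locations through mesh components tagged with slot numbers.
; RemoveCat closes the gap and sends cats to their updated slots via AI movement.
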(event EventBeginPlay
  (bind _asmain_game_instance (Utilities|Casting|CastToMainGameInstance (Game|GetGameInstance)))
  (Variables|/Game/Game/MainGameInstance.MainGameInstance_C|SetQueueManager _asmain_game_instance self))

(event Collision|EventActorBeginOverlap
  (params (OtherActor :type Actor%20Object%20Reference)))

(event EventTick
  (params (DeltaSeconds :type Float%20%28single-precision%29))
  (if (not (Variables|Default|GetPaused))
    (CallFunction|UpdateTimer DeltaSeconds)))

(fn ConstructionScript)

(fn RemoveCat
  (params (cat :type BP%20Cat%20Object%20Reference))
  (if (Utilities|Map|Contains (Variables|Default|GetQueue) cat)
    ;[1 1 1] decremement length of queue
    (bind _result (Math|Integer|DecrementInt (Variables|Default|GetQueueSize))
      (:%20%20
        (Variables|Default|SetQueueSize _result)
        (LocalVariables|SetGapPosition (.Value (Utilities|Map|Find (Variables|Default|GetQueue) cat)))
        ;[1 1 1] Remove from queue map
        (Utilities|Map|Remove (Variables|Default|GetQueue) cat)
        (bind _keys (Utilities|Map|Keys (Variables|Default|GetQueue)))
        (for _array_element _keys ; Move all cats behind the \nqueue gap up a position
          ;[1 1 1] Move all cats that were behind the removed cat up a queue position (temp? add animation later)
          (if (> (.Value (Utilities|Map|Find (Variables|Default|GetQueue) _array_element)) (LocalVariables|GetGapPosition))
            (bind _result_2 (Math|Integer|DecrementInt (.Value (Utilities|Map|Find (Variables|Default|GetQueue) _array_element)))
              (:%20%20
                (Utilities|Map|Add (Variables|Default|GetQueue) _array_element _result_2)))))
        (CallFunction|UpdateWorldPositions)))))

(fn UpdateTimer
  (params (Delta%20Time :type Float%20%28single-precision%29))
  ;[1 1 1] increment time
  (bind _output_get (Variables|Default|SetTimeElapsed (+ Delta%20Time (Variables|Default|GetTimeElapsed))))
  (if (> _output_get (Variables|Default|GetSpawnTime))
    (CallFunction|SpawnCat)))

(fn SpawnCat
  ;[1 1 1] Check that the queue isn't full
  (if (< (Variables|Default|GetQueueSize) (Variables|Default|GetQueueLimit))
    (Variables|Default|SetTimeElapsed 0.0) ; reset time elapsed
    (bind _result (Math|Integer|IncrementInt (Variables|Default|GetQueueSize))
      (:%20%20
        (LocalVariables|SetQueue%20Position _result)
        ;[1 1 1] Spawn and place cat in world
        (bind _type (CallFunction|GetCatType)) ; Randomly generated cat type
        (bind _returnvalue (Game|SpawnActorfromClass _type (Math|Conversions|ToTransform(Vector) (Transformation|GetWorldLocation (Variables|Components|Getspawn%20position))) "AdjustIfPossibleButAlwaysSpawn" 0 0)) ; Spawn cat in front of the door
        ;[1 1 1] Move the spawned cat to the next queue position
        (bind _position (CallFunction|GetWorldPosition (LocalVariables|GetQueue%20Position)))
        (AI|Navigation|SimpleMovetoLocation (AI|GetAIController _returnvalue) _position)
        ;[1 1 1] Add the cat and its queue position to the queue map
        (Utilities|Map|Add (Variables|Default|GetQueue) _returnvalue (LocalVariables|GetQueue%20Position))
        (Audio|PlaySound2D "/Game/Audio/SFX/01_Crystal_Reward__Coming.01_Crystal_Reward__Coming" 1.0 1.0 0.0 0 0)))))

(fn UpdateWorldPositions
  ;[1 1 1] Sets the world position of the cats in the queue, based on their position in the queue
  (bind _keys (Utilities|Map|Keys (Variables|Default|GetQueue)))
  (for _array_element _keys
    (bind _position (CallFunction|GetWorldPosition (.Value (Utilities|Map|Find (Variables|Default|GetQueue) _array_element))))
    (AI|Navigation|MovetoLocation (AI|GetAIController _array_element) _position 0.001 false true false true 0)))

(fn GetWorldPosition
  (params (Queue%20Position :type Integer))
  ;[1 1 1] Gets the world position, given a position in the queue
  (return (Transformation|GetWorldLocation (Utilities|Array|Get(acopy) (Actor|GetComponentsbyTag "/Script/Engine.MeshComponent" (Utilities|String|StringToName (Utilities|String|ToString(Integer) Queue%20Position)))))))

(fn GetCatType
  ;[1 1 1] Gets a type of cat by generating a random number in [0, 1], and checking what probability interval it falls into
  (LocalVariables|SetRandom (Math|Random|RandomFloat))
  (for _array_element (Variables|Default|GetProbabilities)
    (if (Math|Float|InRange(Float) (LocalVariables|GetRandom) (.LowerBound (Utilities|Struct|BreakProbabilityInterval _array_element)) (.UpperBound (Utilities|Struct|BreakProbabilityInterval _array_element)) false)
      (return (.CatType (Utilities|Struct|BreakProbabilityInterval _array_element))))))

(fn SetProbabilities
  (params (Probabilities :type Array%20of%20Spawn%20Probability%20Structures))
  ;[1 1 1] Converts an array of probabilities in [0, 1] to probability intervals with a lower and upper bound
  (for (_array_element _array_index) Probabilities ; Assumes that array is already sorted in \ndescending order by probability.\n\nThis provides a simple optimization for finding what \nprobability range a random number in [0, 1] is in.
    (LocalVariables|SetCat%20Type (.CatType (Utilities|Struct|BreakSpawnProbability _array_element)))
    (LocalVariables|SetProbability (.Probability (Utilities|Struct|BreakSpawnProbability _array_element)))
    (if (== _array_index 0)
      (Utilities|Struct|SetmembersinProbabilityInterval (LocalVariables|GetProbability%20Interval) -0.1) ; Because the lower bound is exclusive, \nwe need to include 0 in the very first interval.
      (else
        (Utilities|Struct|SetmembersinProbabilityInterval (LocalVariables|GetProbability%20Interval) (LocalVariables|GetCumulative%20Probability))))
    (Utilities|Struct|SetmembersinProbabilityInterval (LocalVariables|GetProbability%20Interval) (LocalVariables|GetCat%20Type))
    (bind _output_get (LocalVariables|SetCumulative%20Probability (+ (LocalVariables|GetProbability) (LocalVariables|GetCumulative%20Probability)))) ; Accumulate probability to form upper bound
    (bind _structout (Utilities|Struct|SetmembersinProbabilityInterval (LocalVariables|GetProbability%20Interval) _output_get))
    (Utilities|Array|Add (Variables|Default|GetProbabilities) (|Copy _structout)) ; Finally add the probability interval \nto an array of intervals
  )
  ;[1 1 1] Set upper bound of last interval to 1, in case probabilities don't quite add to 1
  (Utilities|Struct|SetmembersinProbabilityInterval (Utilities|Array|Get(acopy) (Variables|Default|GetProbabilities) (- (Utilities|Array|Length (Variables|Default|GetProbabilities)) 1)) 1.0)
  ;[1 1 1] Checking output
  (for _array_element_2 (Variables|Default|GetProbabilities)
    (Development|PrintString (Utilities|String|Append "L: " (Utilities|String|ToString(Float) (.LowerBound (Utilities|Struct|BreakProbabilityInterval _array_element_2))) ", U:" (Utilities|String|ToString(Float) (.UpperBound (Utilities|Struct|BreakProbabilityInterval _array_element_2))) ", Type:" (Utilities|GetClassDisplayName (.CatType (Utilities|Struct|BreakProbabilityInterval _array_element_2)))) false true "(R=0.000000,G=0.660000,B=1.000000,A=1.000000)" 1e+01)))