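; BP_Table is a clickable restaurant table that seats two cats and tests whether they match.
; AssignCat fills the left then right seat, pulling each cat from the queue, and returns true once paired.
; A click accepted by MainGameInstance stops both patience timers, then runs delayed success or fail reactions before destroying the cats.
; A match also spawns a BP_Coin, limited to one per table.
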(event EventBeginPlay
  (|CallParentFunction) ; This is important for setting up \nappearance of tables
)

(event MouseInput|EventActorOnClicked
  (params (ButtonPressed :type Key%20Structure :default "None"))
  (bind _cat1 (Variables|Default|GetCat1))
  (bind _cat2 (Variables|Default|GetCat2))
  (bind _asmain_game_instance (Utilities|Casting|CastToMainGameInstance (Game|GetGameInstance)))
  (bind _catsassigned (Default|SelectTable _asmain_game_instance self))
  (if _catsassigned
    (Default|StopPatienceTimer _cat1)
    (Default|StopPatienceTimer _cat2)
    (Utilities|FlowControl|Delay 2.0)
    (bind _matchsuccess (Default|CheckMatch _cat1 _cat2))
    (if _matchsuccess
      (Default|OnSuccess _cat1)
      (Default|OnSuccess _cat2)
      (Utilities|FlowControl|Delay 1.0)
      (CallFunction|SpawnCoin)
      (Utilities|FlowControl|Delay 3.0)
      (Actor|DestroyActor _cat1)
      (Actor|DestroyActor _cat2)
      (else
        (Default|OnFail _cat1)
        (Default|OnFail _cat2)
        (Utilities|FlowControl|Delay 4.0)
        (Actor|DestroyActor _cat1)
        (Actor|DestroyActor _cat2)))))

(fn ConstructionScript)

(fn SpawnCoin
  ;[1 1 1] Spawns a coin on top of the table, if there isn't already one
  (if (not (Variables|Default|GetHas%20Coin))
    (Game|SpawnActorfromClass "/Game/Game/BP_Coin.BP_Coin_C" (Math|Conversions|ToTransform(Vector) (Transformation|GetWorldLocation (Variables|Default|GetCoin%20Position))) "Undefined" 0 self 0)
    (Variables|Default|SetHas%20Coin true)))

(fn AssignCat
  (params (ClickedCat :type BP%20Cat%20Object%20Reference))
  (if (Variables|Default|GetCat1Assigned)
    (bind _output_get (Variables|Default|SetCat2 ClickedCat))
    (Default|SitDown _output_get)
    (Default|StopMovement (Variables|Default|GetCat2))
    (Transformation|SetActorLocation (Variables|Default|GetCat2) (Transformation|GetWorldLocation (Variables|Default|GetRIght%20Seat%20Position)) false true)
    (Variables|Default|SetCat1Assigned false)
    (Default|ExitQueue (Variables|Default|GetCat2)) ; moves cats behind cat2 up a queue position
    (return true)
    (else
      (bind _output_get_2 (Variables|Default|SetCat1 ClickedCat))
      (Variables|Default|SetCat1Assigned true)
      (Default|SitDown _output_get_2)
      (Default|StopMovement (Variables|Default|GetCat1))
      (Transformation|SetActorLocation (Variables|Default|GetCat1) (Transformation|GetWorldLocation (Variables|Default|GetLeft%20Seat%20Position)) false true)
      (Default|ExitQueue (Variables|Default|GetCat1)) ; moves cats behind cat 1 up a queue position
      (return false))))